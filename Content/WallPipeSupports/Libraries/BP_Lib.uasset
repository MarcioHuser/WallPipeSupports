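; Function library for the WallPipeSupports mod that repairs pipe support meshes on a given buildable.
; FixPipeMesh only logs when PipelineSupportStatic is valid; otherwise it finds components tagged WallPipe, casts each to FGColoredInstanceMeshProxy and sets SM_PipelineSupport_01 as its mesh.
; A GetPathNameText helper turns object paths into text for the log messages tracing each check and replacement.
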(fn `fixPipeMesh`
  (params (buildable :type "FGBuildable Object Reference"))
  (locals (pipelineSupport_static :type "StaticMesh Object Reference" :default "StaticMesh'/Game/FactoryGame/Buildable/Factory/PipelineSupportWallHole/Mesh/PipelineSupport_static.PipelineSupport_static'"))
  (bind _pipelinesupport_static (`local.pipelineSupport_static`))
  (`SMLBlueprintLibrary.LogInfo` (`KismetTextLibrary.Conv_TextToString` (`|FormatText` "Fixing meshes for build {0}" (`self.getPathNameText` buildable))))
  (if (`KismetSystemLibrary.IsValid` _pipelinesupport_static)
    (`SMLBlueprintLibrary.LogInfo` (`KismetTextLibrary.Conv_TextToString` (`|FormatText` "Mesh {0} is valid" (`self.getPathNameText` _pipelinesupport_static))))
    (else
      (for _array_element (`Actor.GetComponentsByTag` buildable "/Script/Engine.ActorComponent" "WallPipe")
        (bind _asfgcolored_instance_mesh_proxy (cast `FGColoredInstanceMeshProxy` _array_element))
        (`StaticMeshComponent.SetStaticMesh` _asfgcolored_instance_mesh_proxy "/Game/FactoryGame/Buildable/Factory/PipelineSupportWallHole/Mesh/SM_PipelineSupport_01.SM_PipelineSupport_01")
        (`SMLBlueprintLibrary.LogInfo` (`KismetTextLibrary.Conv_TextToString` (`|FormatText` "{object}: Replaced component {component} mesh with {mesh}" (`self.getPathNameText` (`local.buildable`)) (`self.getPathNameText` _asfgcolored_instance_mesh_proxy) (`self.getPathNameText` (`StaticMeshComponent.StaticMesh` _asfgcolored_instance_mesh_proxy)))))))))

(fn `getPathNameText`
  (params (object :type "Object Object Reference"))
  (returns (returnValue :type Text))
  (return (`KismetTextLibrary.Conv_StringToText` (`KismetSystemLibrary.GetPathName` object))))